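; Game mode for Vita that sets up the HUD and tracks gems collected in the level.
; On BeginPlay, InitGame caches the player controller, pawn, game instance and itself, then creates the HUD widget with those references and adds it to the viewport.
; CollectedGem increments the level gem count and broadcasts OnGemCollected.
; UpdateHud forwards refresh requests to the HUD widget.
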(event `self.ReceiveBeginPlay`
  (`self.InitGame`))

(fn `CollectedGem`
  (`/Engine/EditorBlueprintResources/StandardMacros.IncrementInt` (`self.LevelGems`)
    (:`  `
      (`self.OnGemCollected`))))

(fn `InitGame`
  (`|ExecutionSequence`
    (:`then_0`
      ;[1 1 1] Grab reference to things
      (bind _output_get (set `self.PlayerController` (cast `/Game/Vita/Player/PC_VitaPlayerController` (`GameplayStatics.GetPlayerController` 0) :!pure true)))
      (set `self.PlayerPawn` (cast `/Game/Vita/Player/HowieTheBear/PP_VitaPlayerPawn` (`Controller.K2_GetPawn` _output_get) :!pure true))
      (set `self.GameInstance` (cast `/Game/Vita/GI_VitaGameInstance` (`GameplayStatics.GetGameInstance`) :!pure true))
      (bind _asgm_vita_game_mode (cast `/Game/Vita/GM_VitaGameMode` (`GameplayStatics.GetGameMode`)))
      (set `self.GameMode` _asgm_vita_game_mode))
    (:`then_1`
      ;[1 1 1] Create UI elements
      (bind _returnvalue (`|CreateWidget` "/Game/Vita/UI/UI_Hud.UI_Hud_C" (`self.PlayerController`) (`self.GameInstance`) (`self.GameMode`) (`self.PlayerPawn`)))
      (bind _output_get_2 (set `self.UIHud` _returnvalue))
      (`UserWidget.AddToViewport` _output_get_2 0))))

(fn `UpdateHud`
  (`/Game/Vita/UI/UI_Hud.UpdateHUD` (`self.UIHud`))
  (return))

(fn `UserConstructionScript`)