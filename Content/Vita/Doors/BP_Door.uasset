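; BP_Door is a Vita level door that notifies the player pawn via OnDoorEnter when overlapped while open.
; On BeginPlay it opens if keyless or previously opened per the game instance, or if it is next in index order and the player holds keys.
; Activate forces it open, and SetDoorState hides or shows the lock mesh to match.
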(event `self.ReceiveBeginPlay`
  (`self.InitDoor`))

(event `self.Trigger.OnComponentBeginOverlap`
  (params (OverlappedComponent :type "PrimitiveComponent Object Reference") (OtherActor :type "Actor Object Reference") (OtherComp :type "PrimitiveComponent Object Reference") (OtherBodyIndex :type Integer) (bFromSweep :type Boolean) (SweepResult :type "HitResult Structure (by ref)"))
  (bind _aspp_vita_player_pawn (cast `/Game/Vita/Player/HowieTheBear/PP_VitaPlayerPawn` OtherActor))
  (if (`self.IsOpen`)
    (`/Game/Vita/Player/HowieTheBear/PP_VitaPlayerPawn.OnDoorEnter` _aspp_vita_player_pawn self)))

(event `/Game/Vita/BPI_Interactable.Activate`
  (`self.SetDoorState` true))

(fn `InitDoor`
  (`|ExecutionSequence`
    (:`then_0`
      ;[1 1 1] Cache references to things
      (set `self.GameInst` (cast `/Game/Vita/GI_VitaGameInstance` (`GameplayStatics.GetGameInstance`) :!pure true)))
    (:`then_1`
      ;[1 1 1] Determine if we're open/closed
      (if (`self.RequiresKey`)
        ;;[1 1 1] Did we open this door before?
        (if (`/Game/Vita/GI_VitaGameInstance.IsDoorOpened` (`self.GameInst`) (`self.DoorIndex`))
          (set `self.IsOpen` true)
          (else
            ;;[1 1 1] Player has key to open and we're the next door?
            (set `self.IsOpen` (and (>= (`KismetArrayLibrary.Array_Length` (`/Game/Vita/GI_VitaGameInstance.DoorsOpened` (`self.GameInst`))) (`self.DoorIndex`)) (> (`/Game/Vita/GI_VitaGameInstance.Keys` (`self.GameInst`)) 0)))))
        (else
          (set `self.IsOpen` true) ; Doesn't require key, its open
        )))
    (:`then_2`
      (`self.SetDoorState` (`self.IsOpen`)))))

(fn `SetDoorState`
  (params (Open :type Boolean))
  (set `self.IsOpen` Open)
  (`SceneComponent.SetVisibility` (`self.LockMesh`) (not (`self.IsOpen`)) false))

(fn `UserConstructionScript`)