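; BP_HubSwitch is a hub switch that activates an assigned portal actor when the player pawn overlaps its trigger.
; BeginPlay restores the switch state from the game instance's IsHubPortalActive flag.
; The switch shows its state through a dynamic material color and mesh position, and messages the portal only when first switched on.
; Overlap also plays MenuSoundError, which destroys itself when finished so it is heard once.
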(event `self.ReceiveBeginPlay`
  (bind _asgi_vita_game_instance (cast `/Game/Vita/GI_VitaGameInstance` (`GameplayStatics.GetGameInstance`)))
  (set `self.GameInstance` _asgi_vita_game_instance)
  (set `self.IsActive` (`/Game/Vita/GI_VitaGameInstance.IsHubPortalActive` _asgi_vita_game_instance))
  (`self.SetSwitchState` (`self.IsActive`)))

(event `/Game/Vita/BPI_Interactable.Activate`
  (if (not (`self.IsActive`))
    (`self.SetSwitchState` true)
    (`/Engine/EditorBlueprintResources/StandardMacros.IsValid` (`self.PortalActor`)
      (:`Is Valid`
        (message `/Game/Vita/BPI_Interactable.Activate` (`self.PortalActor`)))
      (:`Is Not Valid`
        (`KismetSystemLibrary.PrintString` "Portal Actor is null. Make sure its assigned in the details panel.")))))

(event `self.Trigger.OnComponentBeginOverlap`
  (params (OverlappedComponent :type "PrimitiveComponent Object Reference") (OtherActor :type "Actor Object Reference") (OtherComp :type "PrimitiveComponent Object Reference") (OtherBodyIndex :type Integer) (bFromSweep :type Boolean) (SweepResult :type "HitResult Structure (by ref)"))
  (cast `/Game/Vita/Player/PP_VitaPlayerPawn` OtherActor)
  (`/Game/Vita/BPI_Interactable.Activate`)
  (bind _menu_sound_error (`self.Menu_Sound_Error`)
    (:`then`
      (if (not (`AudioComponent.IsPlaying` _menu_sound_error))
        (`AudioComponent.Play` _menu_sound_error 0.0)
        (add `AudioComponent.OnAudioFinished` _menu_sound_error (delegate `DestroySound`))))
    (:`else`)))

(event `DestroySound`
  (`ActorComponent.K2_DestroyComponent` (`self.Menu_Sound_Error`)))

(event `SetSwitchState`
  (params (Active :type Boolean))
  ;[1 1 1] Activate switch
  (bind _output_get (set `self.IsActive` Active))
  (`MaterialInstanceDynamic.SetVectorParameterValue` (`self.SwitchMID`) "Color" (select `bool` _output_get :`false` (struct :`R` 1.0 :`A` 1.0) :`true` (struct :`G` 1.0 :`A` 1.0) :!type "LinearColor Structure"))
  (`SceneComponent.K2_SetRelativeLocation` (`self.SwitchMesh`) (select `bool` (`self.IsActive`) :`false` (`self.InitialSwitchPos`)) false false))

(fn `UserConstructionScript`
  (bind _switchmesh (`self.SwitchMesh`))
  (`|ExecutionSequence`
    (:`then_0`
      (bind _returnvalue (`PrimitiveComponent.CreateDynamicMaterialInstance` _switchmesh 0 (`PrimitiveComponent.GetMaterial` _switchmesh 0) "None"))
      (bind _output_get (set `self.SwitchMID` _returnvalue))
      (`MaterialInstanceDynamic.SetVectorParameterValue` _output_get "Color" (struct :`R` 1.0 :`A` 1.0)))
    (:`then_1`
      (set `self.InitialSwitchPos` (`SceneComponent.RelativeLocation` (`self.SwitchMesh`))))))