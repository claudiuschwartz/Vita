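; A level portal that sends the Vita player pawn to a target level on overlap while active.
; It opens when the game mode's gem-collected event finds the level gem count has reached the requirement, or through an Activate event.
; SetPortalState swaps visibility between the portal mesh and the inactive sparks and surge cue.
; Portals flagged as hub portals restore their active state from the game instance on BeginPlay and write changes back.
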(event `self.ReceiveBeginPlay`
  (`self.InitPortal`)
  ;[1 1 1] Bind to OnGemCollected
  (add `/Game/Vita/GM_VitaGameMode.OnGemCollected` (`self. GameMode`) (`|CreateDelegate` :!event `OnGemsCollected`)))

(event `OnGemsCollected`
  ;[1 1 1] When we've collected enough gems, portal will open!
  (if (>= (`/Game/Vita/GM_VitaGameMode.LevelGems` (`self. GameMode`)) (`self.GemsRequired`))
    (`self.SetPortalState` true)))

(event `self.Trigger.OnComponentBeginOverlap`
  (params (OverlappedComponent :type "PrimitiveComponent Object Reference") (OtherActor :type "Actor Object Reference") (OtherComp :type "PrimitiveComponent Object Reference") (OtherBodyIndex :type Integer) (bFromSweep :type Boolean) (SweepResult :type "HitResult Structure (by ref)"))
  (bind _aspp_vita_player_pawn (cast `/Game/Vita/Player/PP_VitaPlayerPawn` OtherActor))
  (if (`self.IsActive`)
    (`/Game/Vita/Player/PP_VitaPlayerPawn.OnPortalEnter` _aspp_vita_player_pawn (`self.Goto Level`))))

(event `/Game/Vita/BPI_Interactable.Activate`
  (`self.SetPortalState` true)
  (`AudioComponent.Stop` (`self.PortalSurge_Cue`)))

(fn `InitPortal`
  (`|ExecutionSequence`
    (:`then_0`
      (bind _asgi_vita_game_instance (cast `/Game/Vita/GI_VitaGameInstance` (`GameplayStatics.GetGameInstance`)))
      (set `self.GameInstance` _asgi_vita_game_instance)
      (bind _asgm_vita_game_mode (cast `/Game/Vita/GM_VitaGameMode` (`GameplayStatics.GetGameMode`)))
      (set `self. GameMode` _asgm_vita_game_mode)
      (if (`self.IsHubPortal`)
        (set `self.IsActive` (`/Game/Vita/GI_VitaGameInstance.IsHubPortalActive` (`self.GameInstance`)))))
    (:`then_1`
      (`self.SetPortalState` (`self.IsActive`)))))

(fn `SetPortalState`
  (params (Active :type Boolean))
  (`|ExecutionSequence`
    (:`then_0`
      (bind _output_get (set `self.IsActive` Active))
      (`SceneComponent.SetVisibility` (`self.PortalMesh`) _output_get false)
      (`SceneComponent.SetVisibility` (`self.Sparks`) (not (`self.IsActive`)) false)
      (`SceneComponent.SetVisibility` (`self.PortalSurge_Cue`) (not (`self.IsActive`)) false))
    (:`then_1`
      (if (`self.IsHubPortal`)
        (set `/Game/Vita/GI_VitaGameInstance.IsHubPortalActive` (`self.IsActive`) (`self.GameInstance`))))))

(fn `UserConstructionScript`)