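; BP_Sign is a sign actor in the Vita game that shows multi-line dialogue from its NPCText array.
; Its Box trigger creates a Dialogue widget when the Vita player pawn enters and removes it when the pawn leaves.
; EventDialogueOccurs, not called within this Blueprint, passes NPCText to the widget, reveals it and advances TextRow, or closes it on the last row.
; A DoOnce gates each step and is reset straight afterwards.
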(event `self.Box.OnComponentBeginOverlap`
  (params (OverlappedComponent :type "PrimitiveComponent Object Reference") (OtherActor :type "Actor Object Reference") (OtherComp :type "PrimitiveComponent Object Reference") (OtherBodyIndex :type Integer) (bFromSweep :type Boolean) (SweepResult :type "HitResult Structure (by ref)"))
  (cast `/Game/Vita/Player/HowieTheBear/PP_VitaPlayerPawn` OtherActor)
  (bind _returnvalue (`|CreateWidget` "/Game/Vita/Player/NPC1/Dialogue.Dialogue_C"))
  (bind _output_get (set `self.DialogueUI` _returnvalue))
  (`UserWidget.AddToViewport` _output_get 0))

(event `self.Box.OnComponentEndOverlap`
  (params (OverlappedComponent :type "PrimitiveComponent Object Reference") (OtherActor :type "Actor Object Reference") (OtherComp :type "PrimitiveComponent Object Reference") (OtherBodyIndex :type Integer))
  (bind _dialogueui (`self.DialogueUI`))
  (cast `/Game/Vita/Player/HowieTheBear/PP_VitaPlayerPawn` OtherActor)
  (`/Engine/EditorBlueprintResources/StandardMacros.IsValid` _dialogueui
    (:`Is Valid`
      (`Widget.RemoveFromParent` _dialogueui))))

(event `/Game/Vita/Player/NPC1/NPCInterface.EventDialogueOccurs`
  (bind _returnvalue (+ (`/Game/Vita/Player/NPC1/Dialogue.TextRow` (`self.DialogueUI`)) 1))
  (`/Engine/EditorBlueprintResources/StandardMacros.DoOnce` false :!label _label
    (:`Completed`
      (set `/Game/Vita/Player/NPC1/Dialogue.Text` (`self.NPCText`) (`self.DialogueUI`))
      (`Widget.SetVisibility` (`/Game/Vita/Player/NPC1/Dialogue.TextBlock_0` (`self.DialogueUI`)) "Visible")
      (`Widget.SetVisibility` (`/Game/Vita/Player/NPC1/Dialogue.Image_0` (`self.DialogueUI`)) "Visible")
      (if (> _returnvalue (- (`KismetArrayLibrary.Array_Length` (`self.NPCText`)) 1))
        (`Widget.RemoveFromParent` (`self.DialogueUI`))
        (`self.ResetDialogue`)
        (else
          (set `/Game/Vita/Player/NPC1/Dialogue.TextRow` _returnvalue (`self.DialogueUI`))
          (`self.ResetDialogue`))))))

(event `ResetDialogue`
  (goto _label :!via `Reset`))

(fn `UserConstructionScript`)