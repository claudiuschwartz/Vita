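; Player controller for the Vita game that handles player death and a debug level restart.
; On death it notifies the game instance, unpossesses the pawn, fades the camera to black, then after a short delay asks the Vita game mode to restart the game.
; A debug Alt+X shortcut reloads the current level, tracking the Alt key through a held flag.
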(event `self.ReceiveBeginPlay`
  (set `self.Game Instance` (`/Game/Vita/FL_Vita.REF_GI`)))

(event `Key|X`
  (params (Key :type "Key Structure"))
  ;[1 0.324 0.968] DEBUG - Restart Level (ALT-X)
  (:`Pressed`
    (if (`self.IsHoldingAlt`)
      (bind _returnvalue (`GameplayStatics.GetCurrentLevelName` true))
      (`GameplayStatics.OpenLevel` (`KismetStringLibrary.Conv_StringToName` _returnvalue)))))

(event `Key|LeftAlt`
  (params (Key :type "Key Structure"))
  ;[1 0.324 0.968] DEBUG - Restart Level (ALT-X)
  (:`Pressed`
    (set `self.IsHoldingAlt` true))
  (:`Released`
    (set `self.IsHoldingAlt` false)))

(event `OnDeath`
  (`/Game/Vita/GI_VitaGameInstance.PlayerDied` (`self.Game Instance`))
  (`self.UnPossess`)
  (`PlayerCameraManager.StartCameraFade` :`self` (`self.PlayerCameraManager`) :`ToAlpha` 1.0 :`Duration` 2.0 :`bHoldWhenFinished` true)
  (`KismetSystemLibrary.Delay` 2.1)
  (bind _asgm_vita_game_mode (cast `/Game/Vita/GM_VitaGameMode` (`GameplayStatics.GetGameMode`)))
  (`GameMode.RestartGame` _asgm_vita_game_mode))

(fn `UserConstructionScript`)