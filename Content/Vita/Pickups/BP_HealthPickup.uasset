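; BP_HealthPickup is a health pickup actor that gives health to the Vita player pawn on contact.
; A looping timer at about 30 Hz spins it around yaw, standing in for Tick.
; When its trigger overlaps a PP_VitaPlayerPawn, it passes its HealthAmount to the pawn's PickupHealth, plays a lowered-pitch gem-collect sound and destroys itself.
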(event `self.ReceiveBeginPlay`
  (`KismetSystemLibrary.K2_SetTimerDelegate` (delegate `CustomTick`) 0.033333 true))

(event `CustomTick`
  (`self.K2_AddActorLocalRotation` (`KismetMathLibrary.MakeRotator` 0.0 0.0 5.0)))

(event `self.Trigger.OnComponentBeginOverlap`
  (params (OverlappedComponent :type "PrimitiveComponent Object Reference") (OtherActor :type "Actor Object Reference") (OtherComp :type "PrimitiveComponent Object Reference") (OtherBodyIndex :type Integer) (bFromSweep :type Boolean) (SweepResult :type "HitResult Structure (by ref)"))
  (bind _aspp_vita_player_pawn (cast `/Game/Vita/Player/HowieTheBear/PP_VitaPlayerPawn` OtherActor))
  (`/Game/Vita/Player/HowieTheBear/PP_VitaPlayerPawn.PickupHealth` _aspp_vita_player_pawn (`self.Health Amount`))
  (`GameplayStatics.PlaySoundAtLocation` "/Game/Vita/Sounds/UsedAndInGame/GemCollected.GemCollected" (`self.K2_GetActorLocation`) (struct) 0.5 0.5 0.0 null null null)
  (`self.K2_DestroyActor`))

(fn `UserConstructionScript`
  (`parent.UserConstructionScript`))