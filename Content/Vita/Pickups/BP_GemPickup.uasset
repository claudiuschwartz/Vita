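; BP_GemPickup is a spinning gem collectible for the Vita game that the player pawn picks up by touch.
; A looping timer at roughly 30 Hz drives the yaw rotation in place of Tick.
; Any Trigger overlap plays the GemPickup component, which is stopped at BeginPlay.
; Only a PP_VitaPlayerPawn then receives PickupGem, after which a sound plays at the gem's location and the actor destroys itself.
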(event `self.ReceiveBeginPlay`
  (`AudioComponent.Stop` (`self.GemPickup`))
  (`KismetSystemLibrary.K2_SetTimerDelegate` (delegate `CustomTick`) 0.033333 true))

(event `CustomTick`
  (`self.K2_AddActorLocalRotation` (`KismetMathLibrary.MakeRotator` 0.0 0.0 5.0)))

(event `self.Trigger.OnComponentBeginOverlap`
  (params (OverlappedComponent :type "PrimitiveComponent Object Reference") (OtherActor :type "Actor Object Reference") (OtherComp :type "PrimitiveComponent Object Reference") (OtherBodyIndex :type Integer) (bFromSweep :type Boolean) (SweepResult :type "HitResult Structure (by ref)"))
  (`AudioComponent.Play` (`self.GemPickup`) 0.0)
  (bind _asbp_main_char (cast `/Game/Vita/Player/PP_VitaPlayerPawn` OtherActor))
  (`/Game/Vita/Player/PP_VitaPlayerPawn.PickupGem` _asbp_main_char)
  (`GameplayStatics.PlaySoundAtLocation` "/Game/Vita/Sounds/ui_sound/Menu_Sound_Load_Savefile.Menu_Sound_Load_Savefile" (`self.K2_GetActorLocation`) (struct) 0.7 1.0 0.0 null null null)
  (`self.K2_DestroyActor`))

(fn `UserConstructionScript`
  (`parent.UserConstructionScript`))